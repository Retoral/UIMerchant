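; Player controller for the UI Merchant game that saves and loads the in-game clock and calendar.
; On BeginPlay it caches the game instance and creates a fresh save game object.
; SaveTheGame copies minutes, hours, days and months from the game instance into that object and writes it to the save slot.
; LoadTheGame reads the slot and copies those values back into the game instance.
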(event EventBeginPlay
  (bind _asuimerchant_game_instance_bp (Utilities|Casting|CastToUIMerchant_GameInstance_BP (Game|GetGameInstance)))
  (Variables|Default|SetGame%20Instance _asuimerchant_game_instance_bp)
  (bind _returnvalue (SaveGame|CreateSaveGameObject "/Game/Blueprints/UI_Merchant_SaveGame_BP.UI_Merchant_SaveGame_BP_C"))
  (Variables|Default|SetSave%20Game%20Reference _returnvalue))

(fn ConstructionScript)

(fn SavetheGame
  (bind _game_instance (Variables|Default|GetGame%20Instance))
  (bind _save_game_reference (Variables|Default|GetSave%20Game%20Reference))
  (Variables|/Game/Blueprints/UI_Merchant_SaveGame_BP.UI_Merchant_SaveGame_BP_C|SetMinutes _save_game_reference (Variables|/Game/Blueprints/UIMerchant_GameInstance_BP.UIMerchant_GameInstance_BP_C|GetMinutes _game_instance))
  (Variables|/Game/Blueprints/UI_Merchant_SaveGame_BP.UI_Merchant_SaveGame_BP_C|SetHours _save_game_reference (Variables|/Game/Blueprints/UIMerchant_GameInstance_BP.UIMerchant_GameInstance_BP_C|GetHours _game_instance))
  (Variables|/Game/Blueprints/UI_Merchant_SaveGame_BP.UI_Merchant_SaveGame_BP_C|SetDays _save_game_reference (Variables|/Game/Blueprints/UIMerchant_GameInstance_BP.UIMerchant_GameInstance_BP_C|GetDays _game_instance))
  (Variables|/Game/Blueprints/UI_Merchant_SaveGame_BP.UI_Merchant_SaveGame_BP_C|SetMonths _save_game_reference (Variables|/Game/Blueprints/UIMerchant_GameInstance_BP.UIMerchant_GameInstance_BP_C|GetMonths _game_instance))
  (SaveGame|SaveGametoSlot (Variables|Default|GetSave%20Game%20Reference) (Variables|Default|GetSave%20Slot)))

(fn LoadtheGame
  (bind _game_instance (Variables|Default|GetGame%20Instance))
  (bind _returnvalue (SaveGame|LoadGamefromSlot (Variables|Default|GetSave%20Slot)))
  (bind _asui_merchant_save_game_bp (Utilities|Casting|CastToUI_Merchant_SaveGame_BP _returnvalue))
  (Variables|/Game/Blueprints/UIMerchant_GameInstance_BP.UIMerchant_GameInstance_BP_C|SetMinutes _game_instance (Variables|/Game/Blueprints/UI_Merchant_SaveGame_BP.UI_Merchant_SaveGame_BP_C|GetMinutes _asui_merchant_save_game_bp))
  (Variables|/Game/Blueprints/UIMerchant_GameInstance_BP.UIMerchant_GameInstance_BP_C|SetHours _game_instance (Variables|/Game/Blueprints/UI_Merchant_SaveGame_BP.UI_Merchant_SaveGame_BP_C|GetHours _asui_merchant_save_game_bp))
  (Variables|/Game/Blueprints/UIMerchant_GameInstance_BP.UIMerchant_GameInstance_BP_C|SetDays _game_instance (Variables|/Game/Blueprints/UI_Merchant_SaveGame_BP.UI_Merchant_SaveGame_BP_C|GetDays _asui_merchant_save_game_bp))
  (Variables|/Game/Blueprints/UIMerchant_GameInstance_BP.UIMerchant_GameInstance_BP_C|SetMonths _game_instance (Variables|/Game/Blueprints/UI_Merchant_SaveGame_BP.UI_Merchant_SaveGame_BP_C|GetMonths _asui_merchant_save_game_bp)))